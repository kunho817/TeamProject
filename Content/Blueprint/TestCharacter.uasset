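; TestCharacter is a 2D flipbook character Blueprint with side-to-side movement, an aim toggle and interaction.
; The RightMovement axis flips the sprite through X scale and, outside aim, moves the character and picks walk or idle.
; Right mouse toggles IsAim, switching between the one-shot aim flipbook and looping idle.
; An Interaction event stores an actor, which F casts to handle card key dispensers, puzzle props or a test selection widget.
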(event `self.ReceiveBeginPlay`)

(event `InputAxis|RightMovement`
  (params (AxisValue :type "Float (single-precision)"))
  (bind _paperflipbook (`self.PaperFlipbook`))
  (bind _paperflipbook_2 (`self.PaperFlipbook`))
  (if (`self.IsAim`)
    (if (not (== AxisValue 0.0))
      (`SceneComponent.SetRelativeScale3D` _paperflipbook (`KismetMathLibrary.MakeVector` AxisValue 1.0 1.0)))
    (else
      (if (not (== AxisValue 0.0))
        (`SceneComponent.SetRelativeScale3D` _paperflipbook (`KismetMathLibrary.MakeVector` AxisValue 1.0 1.0)))
      (`self.AddMovementInput` (`KismetMathLibrary.GetForwardVector` (`self.K2_GetActorRotation`)) AxisValue)
      (if (> (`KismetMathLibrary.VSize` (`self.GetVelocity`)) 0.0)
        (`PaperFlipbookComponent.SetFlipbook` _paperflipbook_2 "/Game/Character/C1/Flipbook/C1_Walk.C1_Walk")
        (else
          (`PaperFlipbookComponent.SetFlipbook` _paperflipbook_2 "/Game/Character/C1/Flipbook/C1_Idle.C1_Idle"))))))

(event `Key|F`
  (params (Key :type "Key Structure"))
  (bind _actor (`self.Actor`))
  (:`Pressed`
    (`|ExecutionSequence`
      (:`then_0`
        (bind _ascard_key_dispenser (cast `/Game/Blueprint/Puzzle_Blueprint/CardKey_Dispenser` _actor))
        (bind _count (`/Game/Blueprint/Puzzle_Blueprint/CardKey_Dispenser.Count` _ascard_key_dispenser))
        (`/Engine/EditorBlueprintResources/StandardMacros.IncrementInt` _count
          (:`  `
            (if (== (`/Game/Blueprint/Puzzle_Blueprint/CardKey_Dispenser.Max` _ascard_key_dispenser) _count)
              (message `/Game/Blueprint/Interaction_Interface.Interaction` _actor null)))))
      (:`then_1`
        (bind _aspuzzle_prop (cast `/Game/Blueprint/Puzzle_Blueprint/Puzzle_Prop` _actor))
        (message `/Game/Blueprint/Interaction_Interface.Interaction` _aspuzzle_prop null))
      (:`then_2`
        (cast `/Game/TestInteraction` _actor)
        (bind _returnvalue (`|CreateWidget` "/Game/Blueprint/Selection/Selection_Widget.Selection_Widget_C"))
        (`/Game/Blueprint/Selection/Selection_Widget.Open Selection` _returnvalue "Test")
        (`UserWidget.AddToViewport` _returnvalue 0)))))

(event `Key|RightMouseButton`
  (params (Key :type "Key Structure"))
  (bind _paperflipbook (`self.PaperFlipbook`))
  (:`Pressed`
    (if (and (`self.IsAim`) (not (`PaperFlipbookComponent.IsPlaying` _paperflipbook)))
      (`PaperFlipbookComponent.SetFlipbook` _paperflipbook "/Game/Character/C1/Flipbook/C1_Idle.C1_Idle")
      (`PaperFlipbookComponent.SetLooping` _paperflipbook true)
      (else
        (`PaperFlipbookComponent.SetFlipbook` _paperflipbook "/Game/Character/C1/Flipbook/C1_Aim.C1_Aim")
        (`PaperFlipbookComponent.PlayFromStart` _paperflipbook)
        (`PaperFlipbookComponent.SetLooping` _paperflipbook false)))
    (set `self.IsAim` (not (`self.IsAim`)))))

(event `/Game/Blueprint/Interaction_Interface.Interaction`
  (params (Actor :type "Actor Object Reference"))
  (set `self.Actor` Actor))

(fn `UserConstructionScript`)