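; Bullet is a projectile actor that flies along its forward vector and damages what it hits.
; Tick moves it at constant Speed with a swept SetActorLocation, using the sweep's hit actor for detection.
; IsEnemyAttack selects whether TestCharacter or Enemy receives Damaged, with no destroy after impact.
; Init sets Speed and Damage but leaves its IsEnemy input unused.
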(event `self.ReceiveTick`
  (params (DeltaSeconds :type "Float (single-precision)"))
  (bind _returnvalue (`self.K2_GetActorLocation`))
  (bind _damage (`self.Damage`))
  (bind _sweephitresult (`self.K2_SetActorLocation` (`KismetMathLibrary.VInterpTo_Constant` _returnvalue (+ _returnvalue (* (`self.GetActorForwardVector`) 500.0)) DeltaSeconds (`self.Speed`)) true))
  (if (`self.IsEnemyAttack`)
    (bind (_bblockinghit _binitialoverlap _time _distance _location _impactpoint _normal _impactnormal _physmat _hitactor) (`GameplayStatics.BreakHitResult` _sweephitresult))
    (bind _astest_character (cast `/Game/Blueprint/TestCharacter` _hitactor))
    (`/Game/Blueprint/Interaction_Interface.Damaged` _astest_character _damage)
    (else
      (bind _asenemy (cast `/Game/Blueprint/Enemy/Enemy` _hitactor))
      (`/Game/Blueprint/Interaction_Interface.Damaged` _asenemy _damage))))

(fn `Init`
  (params (Speed :type "Float (double-precision)") (Damage :type "Float (double-precision)") (IsEnemy :type Boolean))
  (set `self.Speed` Speed)
  (set `self.Damage` Damage))

(fn `UserConstructionScript`)