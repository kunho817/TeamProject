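; Puzzle totem prop that registers with a System object and forms part of a numbered sequence.
; Box overlap with TestCharacter sends it an interaction message and, once available, toggles an arrow TextRender.
; Interaction marks the totem available, points the arrow toward the next totem by comparing X positions, and opens the System when its number equals the max count.
; Init also sets the arrow for totem zero.
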(event `self.ReceiveBeginPlay`
  (`/Game/Blueprint/Puzzle_Blueprint/Puzzle_System.AddTotem` (`self.System`) self))

(event `self.Box.OnComponentBeginOverlap`
  (params (OverlappedComponent :type "PrimitiveComponent Object Reference") (OtherActor :type "Actor Object Reference") (OtherComp :type "PrimitiveComponent Object Reference") (OtherBodyIndex :type Integer) (bFromSweep :type Boolean) (SweepResult :type "HitResult Structure (by ref)"))
  (cast `/Game/Blueprint/TestCharacter` OtherActor)
  (set `self.IsOn` true)
  (message `/Game/Blueprint/Interaction_Interface.Interaction` OtherActor self)
  (if (and (`self.IsAvailable`) (`self.IsOn`))
    (`SceneComponent.SetVisibility` (`self.TextRender`) true false)))

(event `self.Box.OnComponentEndOverlap`
  (params (OverlappedComponent :type "PrimitiveComponent Object Reference") (OtherActor :type "Actor Object Reference") (OtherComp :type "PrimitiveComponent Object Reference") (OtherBodyIndex :type Integer))
  (cast `/Game/Blueprint/TestCharacter` OtherActor)
  (set `self.IsOn` false)
  (if (`self.IsAvailable`)
    (`SceneComponent.SetVisibility` (`self.TextRender`) false false)))

(event `/Game/Blueprint/Interaction_Interface.Interaction`
  (params (Actor :type "Actor Object Reference"))
  (bind _system (`self.System`))
  (if (not (and (`self.IsAvailable`) (`self.IsOn`)))
    (`self.Avail`)
    (set `self.IsAvailable` true)
    (bind _result (`/Game/Blueprint/Puzzle_Blueprint/Puzzle_System.GetMaxCount` _system))
    (if (== _result (`self.TotemNum`))
      (`/Game/Blueprint/Puzzle_Blueprint/Puzzle_System.Open` _system))))

(fn `Avail`
  (bind _textrender (`self.TextRender`))
  (bind _totem (`/Game/Blueprint/Puzzle_Blueprint/Puzzle_System.GetNextTotem` (`self.System`) (`self.TotemNum`)))
  (`/Engine/EditorBlueprintResources/StandardMacros.IsValid` _totem
    (:`Is Valid`
      (if (< (- (.x (`self.K2_GetActorLocation`)) (.x (`self.K2_GetActorLocation` _totem))) 0.0)
        (`TextRenderComponent.K2_SetText` _textrender ">")
        (else
          (`TextRenderComponent.K2_SetText` _textrender "<"))))))

(fn `Init`
  (params (TotemNum :type Integer))
  (if (== TotemNum 0)
    (`self.Avail`)))

(fn `UserConstructionScript`)