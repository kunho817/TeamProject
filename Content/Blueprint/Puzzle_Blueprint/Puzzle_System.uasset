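; Puzzle system Blueprint that keeps an indexed registry of totems for a totem puzzle.
; AddTotem stores each totem at its own TotemNum slot, growing the array as needed, then calls Avail on it.
; GetNextTotem returns the totem after a given index and GetMaxCount gives the last index.
; Open only prints a debug string, and BeginPlay is empty.
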(event `self.ReceiveBeginPlay`)

(fn `AddTotem`
  (params (Totem :type "/Game/Blueprint/Puzzle_Blueprint/Puzzle_Prop Object Reference"))
  (`KismetArrayLibrary.Array_Set` (`self.Totem`) (`/Game/Blueprint/Puzzle_Blueprint/Puzzle_Prop.TotemNum` Totem) Totem true)
  (`/Game/Blueprint/Puzzle_Blueprint/Puzzle_Prop.Avail` Totem))

(fn `GetMaxCount`
  (returns (Result :type Integer))
  (return (- (`KismetArrayLibrary.Array_Length` (`self.Totem`)) 1)))

(fn `GetNextTotem`
  (params (Num :type Integer))
  (returns (Totem :type "/Game/Blueprint/Puzzle_Blueprint/Puzzle_Prop Object Reference"))
  (return (`|GetArrayItem` (`self.Totem`) (+ Num 1))))

(fn `Open`
  (`KismetSystemLibrary.PrintString` "Open"))

(fn `UserConstructionScript`)