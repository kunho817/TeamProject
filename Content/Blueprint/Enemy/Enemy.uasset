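; Enemy actor that turns to face the player when in detection range and otherwise wanders along the X axis.
; Tick checks player distance and, in range, flips the sign of X scale to face the player without moving.
; Out of range, a random-delay timer calls Wandering to pick an X target and facing, then Tick moves there with a swept constant-speed interpolation.
; TargetLock is never cleared here, so only one wander target gets chosen.
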(event `self.ReceiveTick`
  (params (DeltaSeconds :type "Float (single-precision)"))
  (bind _returnvalue (`self.K2_GetActorLocation`))
  (bind (_returnvalue_x _returnvalue_y _returnvalue_z) (`KismetMathLibrary.BreakVector` (`self.K2_GetActorLocation`)))
  (bind _returnvalue_2 (`self.K2_GetActorLocation` (`GameplayStatics.GetPlayerPawn` 0)))
  (bind _returnvalue_x_2 (`KismetMathLibrary.BreakVector` (`KismetMathLibrary.GetDirectionUnitVector` _returnvalue _returnvalue_2)))
  (if (<= (`KismetMathLibrary.Vector_Distance` _returnvalue _returnvalue_2) (`self.인식 범위`))
    (`self.SetActorScale3D` (`KismetMathLibrary.MakeVector_NetQuantize` (`KismetMathLibrary.SelectFloat` -3.0 3.0 (< _returnvalue_x_2 0.0)) 3.0 3.0))
    (elif (`self.Target Lock`)
      (`self.K2_SetActorLocation` (`KismetMathLibrary.VInterpTo_Constant` (`self.K2_GetActorLocation`) (`KismetMathLibrary.MakeVector` (`self.Random Move Target`) _returnvalue_y _returnvalue_z) DeltaSeconds 150.0) true)
      (elif (not (`KismetSystemLibrary.K2_IsValidTimerHandle` (`self.Timer`)))
        (bind _returnvalue_3 (`KismetSystemLibrary.K2_SetTimer` null "Wandering" (`KismetMathLibrary.RandomFloatInRange` 1.0 5.0)))
        (set `self.Timer` _returnvalue_3)))))

(fn `UserConstructionScript`)

(fn `Wandering`
  (locals (TempDir :type "Float (double-precision)"))
  (bind _returnvalue_x (`KismetMathLibrary.BreakVector` (`self.K2_GetActorLocation`)))
  (bind _output_get (set `local.TempDir` (`KismetMathLibrary.SelectFloat` -1.0 1.0 (`KismetMathLibrary.RandomBool`))))
  (set `self.Random Move Target` (+ (* _output_get (`KismetMathLibrary.RandomFloatInRange` 0.0 350.0)) _returnvalue_x))
  (set `self.Target Lock` true)
  (`self.SetActorScale3D` (`KismetMathLibrary.MakeVector_NetQuantize` (* _output_get 3.0) 3.0 3.0)))