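; Interactable 2D chest that opens once when it receives an Interaction event.
; On opening, it swaps its Paper2D flipbook to the Chest_Open_Close animation without looping and sets IsOpen to block repeats.
; Its Box overlap sends InteractionMessage to the other actor, passing itself on begin and no target on end.
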(event `/Game/Blueprint/Interaction_Interface.Interaction`
  (params (Actor :type "Actor Object Reference"))
  (bind _paperflipbook (`self.PaperFlipbook`))
  (if (not (`self.IsOpen`))
    (`PaperFlipbookComponent.SetLooping` _paperflipbook false)
    (`PaperFlipbookComponent.SetFlipbook` _paperflipbook "/Game/Blueprint/Interaction/Sprite/Chest_Open_Close.Chest_Open_Close")
    (set `self.IsOpen` true)))

(event `self.Box.OnComponentBeginOverlap`
  (params (OverlappedComponent :type "PrimitiveComponent Object Reference") (OtherActor :type "Actor Object Reference") (OtherComp :type "PrimitiveComponent Object Reference") (OtherBodyIndex :type Integer) (bFromSweep :type Boolean) (SweepResult :type "HitResult Structure (by ref)"))
  (message `/Game/Blueprint/Interaction_Interface.Interaction` OtherActor self))

(event `self.Box.OnComponentEndOverlap`
  (params (OverlappedComponent :type "PrimitiveComponent Object Reference") (OtherActor :type "Actor Object Reference") (OtherComp :type "PrimitiveComponent Object Reference") (OtherBodyIndex :type Integer))
  (message `/Game/Blueprint/Interaction_Interface.Interaction` OtherActor null))

(fn `UserConstructionScript`)