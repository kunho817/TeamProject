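; PC_PlayerController is a player controller that sets up the player's data and HUD and handles menu and level-loading input.
; On BeginPlay it caches the TP_PlayerState, calls SetData on it, then creates the WB_PlayerHUD widget.
; The Inventory action opens the HUD's player menu.
; A hard-wired Q key calls DataUpdate on the player state, then shows a loading screen initialized with the hard-coded name Downtown_A1.
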(event `Key|Q`
  (params (Key :type "Key Structure"))
  (:`Pressed`
    (`/Game/Blueprints/System_Blueprint/TP_PlayerState.DataUpdate` (`self.PS`))
    (bind _returnvalue (`|CreateWidget` "/Game/Blueprints/WidgetBlueprints/WB_LoadingScreen.WB_LoadingScreen_C"))
    (`/Game/Blueprints/WidgetBlueprints/WB_LoadingScreen.Init` _returnvalue "Downtown_A1")
    (`UserWidget.AddToViewport` _returnvalue 0)))

(event `self.ReceiveBeginPlay`
  (bind _astp_player_state (cast `/Game/Blueprints/System_Blueprint/TP_PlayerState` (`GameplayStatics.GetPlayerState` 0)))
  (bind _output_get (set `self.PS` _astp_player_state))
  (`/Game/Blueprints/System_Blueprint/TP_PlayerState.SetData` _output_get)
  (bind _returnvalue (`|CreateWidget` "/Game/Blueprints/WidgetBlueprints/WB_PlayerHUD.WB_PlayerHUD_C"))
  (bind _output_get_2 (set `self.HUD` _returnvalue))
  (`UserWidget.AddToViewport` _output_get_2 0))

(event `InputAction|Inventory`
  (params (Key :type "Key Structure"))
  (:`Pressed`
    (`/Game/Blueprints/WidgetBlueprints/WB_PlayerHUD.DisplayPlayerMenu` (`self.HUD`))))

(fn `UserConstructionScript`)