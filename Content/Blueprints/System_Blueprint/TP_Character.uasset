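; Player character for a 2D Paper2D game, handling side-on movement, aimed shooting, interaction and damage.
; Input flips and animates the flipbook, blocks walking while aiming, and drives ShootingSystemBP for direction and firing.
; Tick uses flipbook playback to end shots and reversed-aim exits, halving shot animation speed without a "gun" inventory item.
; F dispatches by cast on the stored interaction actor, while damage is forwarded to TP_PlayerState.
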(event `self.ReceiveBeginPlay`
  (set `/Game/Blueprints/System_Blueprint/ShootingSystem_BP.Arrow` (`self.Arrow1`) (`self.ShootingSystem_BP`))
  (set `self.HP` (`self.MaxHP`)))

(event `InputAxis|RightMovement`
  (params (AxisValue :type "Float (single-precision)"))
  (bind _paperflipbook (`self.PaperFlipbook`))
  (bind _paperflipbook_2 (`self.PaperFlipbook`))
  (`/Game/Blueprints/System_Blueprint/ShootingSystem_BP.ChangeShootLine` (`self.ShootingSystem_BP`) AxisValue)
  (if (`self.IsAim`)
    (if (not (== AxisValue 0.0))
      (`SceneComponent.SetRelativeScale3D` _paperflipbook (`KismetMathLibrary.MakeVector` AxisValue 1.0 1.0)))
    (else
      (if (not (== AxisValue 0.0))
        (`SceneComponent.SetRelativeScale3D` _paperflipbook (`KismetMathLibrary.MakeVector` AxisValue 1.0 1.0)))
      (`self.AddMovementInput` (`KismetMathLibrary.GetForwardVector` (`self.K2_GetActorRotation`)) AxisValue)
      (if (> (`KismetMathLibrary.VSize` (`self.GetVelocity`)) 0.0)
        (`PaperFlipbookComponent.SetFlipbook` _paperflipbook_2 "/Game/Sprites/CharacterSprite/C1/Flipbook/C1_Walk.C1_Walk")
        (else
          (`PaperFlipbookComponent.SetFlipbook` _paperflipbook_2 "/Game/Sprites/CharacterSprite/C1/Flipbook/C1_Idle.C1_Idle"))))))

(event `Key|F`
  (params (Key :type "Key Structure"))
  (bind _actor (`self.Actor`))
  (:`Pressed`
    (`|ExecutionSequence`
      (:`then_0`
        (bind _ascard_key_dispenser (cast `/Game/Blueprints/System_Blueprint/Puzzle_Blueprint/CardKey_Dispenser` _actor))
        (bind _count (`/Game/Blueprints/System_Blueprint/Puzzle_Blueprint/CardKey_Dispenser.Count` _ascard_key_dispenser))
        (`/Engine/EditorBlueprintResources/StandardMacros.IncrementInt` _count
          (:`  `
            (if (== (`/Game/Blueprints/System_Blueprint/Puzzle_Blueprint/CardKey_Dispenser.Max` _ascard_key_dispenser) _count)
              (message `/Game/Blueprints/System_Blueprint/Interaction_Interface.Interaction` _actor null)))))
      (:`then_1`
        (bind _aspuzzle_prop (cast `/Game/Blueprints/System_Blueprint/Puzzle_Blueprint/Puzzle_Prop` _actor))
        (message `/Game/Blueprints/System_Blueprint/Interaction_Interface.Interaction` _aspuzzle_prop null))
      (:`then_2`
        (cast `/Game/Blueprints/System_Blueprint/Interaction_NPC` _actor)
        (set `PlayerController.bShowMouseCursor` true (`GameplayStatics.GetPlayerController` 0))
        (bind _returnvalue (`|CreateWidget` "/Game/Blueprints/System_Blueprint/Selection/Selection_Widget.Selection_Widget_C"))
        (`UserWidget.AddToViewport` _returnvalue 0))
      (:`then_3`
        (bind _aschest_bp (cast `/Game/Blueprints/System_Blueprint/Interaction/Chest_BP` _actor))
        (`/Game/Blueprints/System_Blueprint/Interaction_Interface.Interaction` _aschest_bp self))
      (:`then_4`
        (bind _asbp_bunker_exit (cast `/Game/Blueprints/System_Blueprint/Interaction/BP_Bunker_Exit` _actor))
        (`/Game/Blueprints/System_Blueprint/Interaction_Interface.Interaction` _asbp_bunker_exit null))
      (:`then_5`
        (bind _asbp_combine (cast `/Game/Blueprints/System_Blueprint/Interaction/BP_Combine` _actor))
        (`/Game/Blueprints/System_Blueprint/Interaction_Interface.Interaction` _asbp_combine self)))))

(event `Key|RightMouseButton`
  (params (Key :type "Key Structure"))
  (bind _paperflipbook (`self.PaperFlipbook`))
  (:`Pressed`
    (if (and (`self.IsAim`) (not (`PaperFlipbookComponent.IsPlaying` _paperflipbook)))
      (`PaperFlipbookComponent.SetFlipbook` _paperflipbook "/Game/Sprites/CharacterSprite/C1/Flipbook/C1_Aim.C1_Aim")
      (`PaperFlipbookComponent.ReverseFromEnd` _paperflipbook)
      (set `self.ToIdle` true)
      (else
        (`PaperFlipbookComponent.SetFlipbook` _paperflipbook "/Game/Sprites/CharacterSprite/C1/Flipbook/C1_Aim.C1_Aim")
        (`PaperFlipbookComponent.PlayFromStart` _paperflipbook)
        (`PaperFlipbookComponent.SetLooping` _paperflipbook false)
        (set `self.IsAim` true)))))

(event `Key|LeftMouseButton`
  (params (Key :type "Key Structure"))
  (bind _paperflipbook (`self.PaperFlipbook`))
  (:`Pressed`
    (if (`self.IsAim`)
      (if (not (`self.IsShoot`))
        (`PaperFlipbookComponent.SetFlipbook` _paperflipbook "/Game/Sprites/CharacterSprite/C1/Flipbook/C1_Shoot.C1_Shoot")
        (`PaperFlipbookComponent.PlayFromStart` _paperflipbook)
        (set `self.IsShoot` true)
        (`/Game/Blueprints/System_Blueprint/ShootingSystem_BP.Shoot` (`self.ShootingSystem_BP`))))))

(event `/Game/Blueprints/System_Blueprint/Interaction_Interface.Interaction`
  (params (Actor :type "Actor Object Reference"))
  (set `self.Actor` Actor))

(event `self.ReceiveTick`
  (params (DeltaSeconds :type "Float (single-precision)"))
  (bind _paperflipbook (`self.PaperFlipbook`))
  (bind _paperflipbook_2 (`self.PaperFlipbook`))
  (bind _paperflipbook_3 (`self.PaperFlipbook`))
  (`|ExecutionSequence`
    (:`then_0`
      (if (and (== (`PaperFlipbookComponent.GetFlipbook` _paperflipbook_3) "/Game/Sprites/CharacterSprite/C1/Flipbook/C1_Shoot.C1_Shoot") (not (`PaperFlipbookComponent.IsPlaying` _paperflipbook_3)))
        (set `self.IsShoot` false)))
    (:`then_1`
      (if (and (`self.ToIdle`) (not (`PaperFlipbookComponent.IsPlaying` _paperflipbook_3)))
        (`PaperFlipbookComponent.SetFlipbook` _paperflipbook "/Game/Sprites/CharacterSprite/C1/Flipbook/C1_Idle.C1_Idle")
        (`PaperFlipbookComponent.PlayFromStart` _paperflipbook)
        (`PaperFlipbookComponent.SetLooping` _paperflipbook true)
        (set `self.ToIdle` false)
        (set `self.IsAim` false)))
    (:`then_2`
      (if (`self.IsShoot`)
        (bind _bool (`self.IsNewGun`))
        (if _bool
          (`PaperFlipbookComponent.SetPlayRate` _paperflipbook_2 1.0)
          (else
            (`PaperFlipbookComponent.SetPlayRate` _paperflipbook_2 0.5)))))))

(event `/Game/Blueprints/System_Blueprint/Interaction_Interface.Damaged`
  (params (Damage :type "Float (double-precision)"))
  (bind _astp_player_state (cast `/Game/Blueprints/System_Blueprint/TP_PlayerState` (`Controller.PlayerState` (`GameplayStatics.GetPlayerController` 0))))
  (`/Game/Blueprints/System_Blueprint/TP_PlayerState.Damaged` _astp_player_state Damage))

(fn `ChangeShootLine`
  (params (in :type "Float (double-precision)"))
  (bind _arrow1 (`self.Arrow1`))
  (`SceneComponent.K2_SetRelativeRotation` _arrow1 (`KismetMathLibrary.MakeRotator` (.roll (`SceneComponent.RelativeRotation` _arrow1)) (.pitch (`SceneComponent.RelativeRotation` _arrow1)) (`KismetMathLibrary.SelectFloat` (.yaw (`SceneComponent.RelativeRotation` _arrow1)) (`KismetMathLibrary.SelectFloat` 0.0 180.0 (== in 1.0)) (== in 0.0))) false false))

(fn `IsNewGun`
  (returns (Bool :type Boolean))
  (bind (_index _foundslot) (`/Game/Blueprints/Inventory/BP_AC_Inventory.FindSlot` (`self.BP_AC_Inventory`) "gun"))
  (return _foundslot))

(fn `UserConstructionScript`)