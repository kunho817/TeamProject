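; TP_PlayerState is a player state that tracks HP and syncs it, along with inventory content, with the TP_GI game instance.
; SetData loads HP from the game instance and copies its stored Content into the first player's TestCharacter inventory component; DataUpdate writes both back.
; Damaged subtracts damage only when the remaining HP stays above zero, so a lethal hit leaves HP unchanged.
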(fn `Damaged`
  (params (Damage :type "Float (double-precision)"))
  (bind _returnvalue (- (`self.HP`) Damage))
  (if (not (<= _returnvalue 0.0))
    (set `self.HP` _returnvalue)))

(fn `DataUpdate`
  (bind _astp_gi (cast `/Game/Blueprints/System_Blueprint/TP_GI` (`GameplayStatics.GetGameInstance`)))
  (`/Game/Blueprints/System_Blueprint/TP_GI.SetHP` _astp_gi (`self.HP`))
  (bind _astest_character (cast `/Game/Blueprints/System_Blueprint/TestCharacter` (`GameplayStatics.GetPlayerPawn` 0)))
  (set `/Game/Blueprints/System_Blueprint/TP_GI.Content` (`/Game/Blueprints/Inventory/BP_AC_Inventory.Content` (`/Game/Blueprints/System_Blueprint/TestCharacter.BP_AC_Inventory` _astest_character)) _astp_gi))

(fn `SetData`
  (bind _astp_gi (cast `/Game/Blueprints/System_Blueprint/TP_GI` (`GameplayStatics.GetGameInstance`)))
  (bind _hp (`/Game/Blueprints/System_Blueprint/TP_GI.GetHP` _astp_gi))
  (set `self.HP` _hp)
  (bind _astest_character (cast `/Game/Blueprints/System_Blueprint/TestCharacter` (`GameplayStatics.GetPlayerPawn` 0)))
  (set `/Game/Blueprints/Inventory/BP_AC_Inventory.Content` (`/Game/Blueprints/System_Blueprint/TP_GI.Content` _astp_gi) (`/Game/Blueprints/System_Blueprint/TestCharacter.BP_AC_Inventory` _astest_character)))

(fn `UserConstructionScript`)