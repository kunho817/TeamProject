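; TP_GI is a game-instance-style Blueprint, judging by its name, that stores player HP and a title-state flag.
; Simple accessors set and return HP and return the OnTitle flag.
; SetMaxHP fills HP from MaxHP only while the FristLogin flag is true, then clears the flag so later calls leave HP unchanged.
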(fn `Get OnTitle`
  (returns (bool :type Boolean))
  (return (`self.OnTitle`)))

(fn `GetHP`
  (returns (HP :type "Float (double-precision)"))
  (return (`self.HP`)))

(fn `SetHP`
  (params (HP :type "Float (double-precision)"))
  (set `self.HP` HP))

(fn `SetMaxHP`
  (if (`self.FristLogin`)
    (set `self.HP` (`self.MaxHP`))
    (set `self.FristLogin` false)))