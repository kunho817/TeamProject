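; Shooting system for a side-view game that fires hitscan shots from an Arrow, which ChangeShootLine flips left or right.
; Shoot, blocked while paused, plays a gunshot, spawns a bullet trail and line-traces with random vertical spread.
; Hits spawn an impact effect at a fixed Y depth with a random flipbook.
; Enemies and player characters receive Damage through DamagedMessage, while obstacles only print a debug string.
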(fn `ChangeShootLine`
  (params (in :type "Float (double-precision)"))
  (bind _arrow (`self.Arrow`))
  (`SceneComponent.K2_SetRelativeRotation` _arrow (`KismetMathLibrary.MakeRotator` (.roll (`SceneComponent.RelativeRotation` _arrow)) (.pitch (`SceneComponent.RelativeRotation` _arrow)) (`KismetMathLibrary.SelectFloat` (.yaw (`SceneComponent.RelativeRotation` _arrow)) (`KismetMathLibrary.SelectFloat` 0.0 180.0 (== in 1.0)) (== in 0.0))) false false))

(fn `Shoot`
  (locals (Temp :type "Vector Structure"))
  (bind _damage (`self.Damage`))
  (bind _arrow (`self.Arrow`))
  (bind _returnvalue (`SceneComponent.K2_GetComponentLocation` _arrow))
  (bind _astp_game_mode (cast `/Game/Blueprints/System_Blueprint/TP_GameMode` (`GameplayStatics.GetGameMode`)))
  (if (not (`/Game/Blueprints/System_Blueprint/TP_GameMode.Pause` _astp_game_mode))
    (`GameplayStatics.PlaySound2D` "/Game/Audio/1911-_45-ACP-Close-Single-Gunshot-A-www_fesliyanstudios_com.1911-_45-ACP-Close-Single-Gunshot-A-www_fesliyanstudios_com" (`/Game/Blueprints/System_Blueprint/TP_GameMode.Volume` _astp_game_mode) 1.0 0.0 null null false)
    (bind _output_get (set `local.Temp` (`KismetMathLibrary.MakeVector` (.x (+ (* (`SceneComponent.GetForwardVector` _arrow) 1000.0) _returnvalue)) (.y (+ (* (`SceneComponent.GetForwardVector` _arrow) 1000.0) _returnvalue)) (+ (.z (+ (* (`SceneComponent.GetForwardVector` _arrow) 1000.0) _returnvalue)) (`KismetMathLibrary.RandomFloatInRange` -50.0 50.0)))))
    (bind _returnvalue_2 (`KismetMathLibrary.FindLookAtRotation` _returnvalue _output_get))
    (`|SpawnActorFromClass` "/Game/Sprites/CharacterSprite/Bullet/Bullet_Trail.Bullet_Trail_C" (`KismetMathLibrary.MakeTransform` _returnvalue _returnvalue_2) "Undefined" "OverrideRootScale" null null)
    (bind (_outhit _returnvalue_3) (`KismetSystemLibrary.LineTraceSingle` :`Start` _returnvalue :`End` _output_get :`TraceChannel` "TraceTypeQuery3" :`DrawTime` 1.0))
    (if _returnvalue_3
      (bind (_bblockinghit _binitialoverlap _time _distance _location _impactpoint _normal _impactnormal _physmat _hitactor) (`GameplayStatics.BreakHitResult` _outhit))
      (bind _returnvalue_4 (`|SpawnActorFromClass` "/Game/Sprites/CharacterSprite/Bullet/Bullet_Damaged.Bullet_Damaged_C" (`KismetMathLibrary.MakeTransform` (`KismetMathLibrary.MakeVector_NetQuantize` (.x _impactpoint) 30.0 (.z _impactpoint)) _returnvalue_2) "Undefined" "OverrideRootScale" null null))
      (`/Game/Sprites/CharacterSprite/Bullet/Bullet_Damaged.SetFlip` _returnvalue_4 (select `bool` (`KismetMathLibrary.RandomBool`) :`false` "/Game/Sprites/CharacterSprite/Bullet/flipbook/shot-expert1.shot-expert1" :`true` "/Game/Sprites/CharacterSprite/Bullet/flipbook/shot-expert2.shot-expert2" :!type "PaperFlipbook Object Reference"))
      (cast `/Game/Blueprints/System_Blueprint/Obstacle/Obstacle_BP` _hitactor
        (:`then`
          (`KismetSystemLibrary.PrintString` "obstacle" true true (struct :`A` 1.0)))
        (:`CastFailed`
          (bind _asenemy (cast `/Game/Blueprints/System_Blueprint/Enemy/Enemy` _hitactor)
            (:`then`
              (message `/Game/Blueprints/System_Blueprint/Interaction_Interface.Damaged` _asenemy _damage))
            (:`CastFailed`
              (bind _astp_character (cast `/Game/Blueprints/System_Blueprint/TP_Character` _hitactor))
              (message `/Game/Blueprints/System_Blueprint/Interaction_Interface.Damaged` _astp_character _damage))))))))