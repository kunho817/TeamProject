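; Inventory actor component that stores items as stackable slots of item ID and quantity in a Content array.
; AddToInventory places items one unit at a time, topping up matching stacks before filling empty slots, and returns success and leftover quantity.
; Stack limits come from the DT_Item data table, and a quantity of zero marks a slot empty.
; RemoveFromInventory is an empty stub.
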(fn `AddToInventory`
  (params (ItemID :type Name) (Quantity :type Integer))
  (returns (Success :type Boolean) (QuantityRemaining :type Integer))
  (locals (Local_QuantityRemaining :type Integer) (Local_HasFailed :type Boolean))
  (set `local.Local_QuantityRemaining` Quantity)
  (while (== (> (`local.Local_QuantityRemaining`) 0) (not (`local.Local_HasFailed`)))
    (bind (_index _foundslot) (`self.FindSlot` (`local.ItemID`)))
    (if _foundslot
      (`self.AddToStack` _index 1)
      (`/Engine/EditorBlueprintResources/StandardMacros.DecrementInt` (`local.Local_QuantityRemaining`))
      (elif (`self.AnyEmptySlotsAvailable`)
        (bind _success (`self.CreateNewStack` (`local.ItemID`) 1))
        (if _success
          (`/Engine/EditorBlueprintResources/StandardMacros.DecrementInt` (`local.Local_QuantityRemaining`))
          (else
            (set `local.Local_HasFailed` true)))
        (else
          (set `local.Local_HasFailed` true)))))
  (return (not (`local.Local_HasFailed`)) (`local.Local_QuantityRemaining`)))

(fn `AddToStack`
  (params (Index :type Integer) (Quantity :type Integer))
  (bind (_output_itemid _output_quantity) (break `/Game/Blueprints/Inventory/Str_Slot` (`|GetArrayItem` (`self.Content`) Index)))
  (`KismetArrayLibrary.Array_Set` (`self.Content`) Index (make `/Game/Blueprints/Inventory/Str_Slot` _output_itemid (+ _output_quantity Quantity))))

(fn `AnyEmptySlotsAvailable`
  (returns (HasEmptySlot :type Boolean) (EmptyIndex :type Integer))
  (for (_array_element _array_index) (`self.Content`)
    (if (== (`.Quantity_5_F0742FF24B1821A21193BE8C175C888A` (break `/Game/Blueprints/Inventory/Str_Slot` _array_element)) 0)
      (return true _array_index)))
  (return false -1))

(fn `CreateNewStack`
  (params (ItemID :type Name) (Quantity :type Integer))
  (returns (Success :type Boolean))
  (bind (_hasemptyslot _emptyindex) (`self.AnyEmptySlotsAvailable`))
  (if _hasemptyslot
    (`KismetArrayLibrary.Array_Set` (`self.Content`) _emptyindex (make `/Game/Blueprints/Inventory/Str_Slot` ItemID Quantity))
    (return true)
    (else
      (return false))))

(fn `FindSlot`
  (params (ItemID :type Name))
  (returns (Index :type Integer) (FoundSlot :type Boolean))
  (for (_array_element _array_index) (`self.Content`)
    (bind (_itemid _quantity) (break `/Game/Blueprints/Inventory/Str_Slot` _array_element))
    (if (== _itemid (`local.ItemID`))
      (if (< _quantity (`self.GetMaxStackSize` (`local.ItemID`)))
        (return _array_index true))))
  (return -1 false))

(fn `GetMaxStackSize`
  (params (ItemID :type Name))
  (returns (StackSize :type Integer))
  (bind _returnvalue (`|GetDataTableRow` "/Game/Blueprints/Inventory/DT_Item.DT_Item" ItemID)
    (:`then`
      (return (`.StackSize_15_B54C0596453697096E6374A8F35D04E9` (break `/Game/Blueprints/Inventory/Str_Item` _returnvalue))))
    (:`RowNotFound`
      (return -1))))

(fn `RemoveFromInventory`)